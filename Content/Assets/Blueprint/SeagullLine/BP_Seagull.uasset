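; BP_Seagull is an actor that flies along a spline path, presumably as an ambient seagull.
; On BeginPlay it falls back to the first BP_SplinePath in the level if no path is assigned, then starts a timeline scaled by CircuitTimeSeconds.
; Each timeline update maps the track value to a distance along the spline and sets the actor's world location and rotation there, with a fixed enlarged scale.
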(event Custom|Move%20Object
  (bind _splinepath (Variables|Default|GetSplinePath))
  (bind _spline (Variables|/Game/Assets/Blueprint/SeagullLine/BP_SplinePath.BP_SplinePath_C|GetSpline _splinepath))
  (Components|Timeline|SetPlayRate (Variables|Default|GetMoving%20Object) (/ 1.0 (Variables|Default|GetCircuit%20Time%20%28seconds%29)))
  (bind _move_track (Timeline|Moving%20Object Play)
    (:Update
      (Transformation|SetActorTransform (Math|Transform|MakeTransform (Spline|GetLocationatDistanceAlongSpline _spline (Math|Float|Lerp 0.0 (Spline|GetSplineLength (Variables|/Game/Assets/Blueprint/SeagullLine/BP_SplinePath.BP_SplinePath_C|GetSpline (Variables|Default|GetSplinePath))) _move_track) "World") (Spline|GetRotationatDistanceAlongSpline _spline (Math|Float|Lerp 0.0 (Spline|GetSplineLength (Variables|/Game/Assets/Blueprint/SeagullLine/BP_SplinePath.BP_SplinePath_C|GetSpline (Variables|Default|GetSplinePath))) _move_track) "World") "5.000000,5.000000,5.000000")))))

(event EventBeginPlay
  (Utilities|IsValid (Variables|Default|GetSplinePath)
    (:Is%20Valid
      _)
    (:Is%20Not%20Valid
      (bind _returnvalue (Actor|GetActorOfClass "/Game/Assets/Blueprint/SeagullLine/BP_SplinePath.BP_SplinePath_C"))
      (Variables|Default|SetSplinePath _returnvalue)))
  (CallFunction|MoveObject))

(fn ConstructionScript)