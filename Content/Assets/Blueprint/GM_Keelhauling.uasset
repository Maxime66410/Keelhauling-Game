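; Game mode for the Keelhauling minigame, a turn-based point contest between player and AI with cannons.
; On BeginPlay it finds the camera and both cannon spawners by display name and adds the in-game UI.
; A self-rescheduling timer runs delayed AI turns: random point gains, then a rare cannon attack, guaranteed on hard, that shifts points, before passing the turn.
; Tick prints both scores; StartGame is empty.
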(event Custom|StartGame)

(event Custom|SetupMap
  ;[1 1 1] Setup Map
  ;;[1 1 1] Setup Camera
  (bind _outactors (Actor|GetAllActorsOfClass "/Script/Engine.CameraActor"))
  (bind _array_element (Utilities|Array|ForEachLoopwithBreak _outactors :!label _label)
    (:LoopBody
      (if (Utilities|Enum|Equal(Enum) (Utilities|GetDisplayName _array_element) "CameraActorForGame")
        (Variables|Default|SetMain%20Camera _array_element)
        (goto _label Break)))
    (:Completed
      ;;[1 1 1] Setup UI
      (Game|Player|SetViewTargetwithBlend (Game|GetPlayerController 0) (Variables|Default|GetMain%20Camera) 0.0 "VTBlend_Linear" 0.0 false)
      (bind _returnvalue (UserInterface|CreateWidget "/Game/Assets/Blueprint/UI/UI_InGame.UI_InGame_C"))
      (Variables|Default|SetUIGAME _returnvalue)
      (UserInterface|Viewport|AddtoViewport _returnvalue 0)
      ;;[1 1 1] Setup cannon
      (bind _outactors_2 (Actor|GetAllActorsOfClass "/Game/Assets/Blueprint/Projectile/BP_SpawnCannonBall.BP_SpawnCannonBall_C"))
      (bind _array_element_2 (Utilities|Array|ForEachLoopwithBreak _outactors_2)
        (:LoopBody
          (if (Utilities|Enum|Equal(Enum) (Utilities|GetDisplayName _array_element_2) "BP_SpawnCannonBallPlayer")
            (Variables|Default|SetCannonPlayer _array_element_2)
            (elif (Utilities|Enum|Equal(Enum) (Utilities|GetDisplayName _array_element_2) "BP_SpawnCannonBallAI")
              (Variables|Default|SetCannonAI _array_element_2))))))))

(event Custom|TourAI
  (if (not (Variables|Default|GetTourPlayer))
    (Utilities|FlowControl|Delay 2.0)
    ;[1 1 1] AI can get 65% to chance get new points
    (if (Math|Random|RandomBoolwithWeight 0.65)
      (Variables|Default|SetPointAI (+ (Variables|Default|GetPointAI) (Utilities|Select :Index (Math|Random|RandomIntegerinRange 0 4) :Option%200 2 :Option%201 4 :Option%202 6 :Option%203 8 :Option%204 20))))
    (Utilities|FlowControl|Delay 2.0)
    ;[1 1 1] AI can Attack player with 5% to chance (10% with hard mode)
    (if (select (Variables|Default|GetDifficultyHard) (Math|Random|RandomBoolwithWeight 1.0) (Math|Random|RandomBoolwithWeight 0.05))
      (Default|SpawnCannonBall (Variables|Default|GetCannonAI))
      (Variables|Default|SetPointPlayer (- (Variables|Default|GetPointPlayer) 50))
      (Variables|Default|SetPointAI (+ (Variables|Default|GetPointAI) 25)))
    (Utilities|FlowControl|Delay 2.0)
    ;[1 1 1] Pass Round
    (Variables|Default|SetTourPlayer true)
    (Utilities|Time|SetTimerbyEvent (delegate Custom|TourAI) 1.0)
    (else
      (Utilities|Time|SetTimerbyEvent (delegate Custom|TourAI) 1.0))))

(event EventBeginPlay
  (CallFunction|SetupMap)
  (CallFunction|TourAI))

(event EventTick
  (params (DeltaSeconds :type Float%20%28single-precision%29))
  (Development|PrintString (Utilities|String|Append (Utilities|String|ToString(Integer) (Variables|Default|GetPointPlayer)) " | " (Utilities|String|ToString(Integer) (Variables|Default|GetPointAI))) true true "(R=0.000000,G=0.660000,B=1.000000,A=1.000000)" 0.005))

(fn ConstructionScript)