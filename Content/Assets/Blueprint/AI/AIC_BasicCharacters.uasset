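; AI controller for BP_BasicCharacters pawns that starts the BT_BasicCharacters behavior tree on BeginPlay and caches its blackboard.
; On possess, it stores the cast pawn and waits briefly.
; It then writes the world location of the pawn's ArrayElement actor into the ActorVector blackboard key, a one-time snapshot rather than a continuous update.
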(event EventPossess
  (params (PossessedPawn :type Pawn%20Object%20Reference))
  (bind _asbp_basic_characters (Utilities|Casting|CastToBP_BasicCharacters PossessedPawn))
  (bind _output_get (Variables|Default|SetAs%20BP%20Basic%20Characters _asbp_basic_characters))
  (Utilities|FlowControl|Delay 0.2)
  (AI|Components|Blackboard|SetValueasVector (Variables|Default|GetBlackboard%20Component) (Utilities|Name|MakeLiteralName "ActorVector") (Transformation|GetWorldLocation (Variables|/Script/Engine.Actor|GetRootComponent (Variables|/Game/Assets/Blueprint/AI/BP_BasicCharacters.BP_BasicCharacters_C|GetArray%20Element _output_get)))))

(event EventBeginPlay
  (AI|RunBehaviorTree "/Game/Assets/Blueprint/AI/BT_BasicCharacters.BT_BasicCharacters")
  (Variables|Default|SetBlackboard%20Component (AI|GetBlackboard 0)))

(fn ConstructionScript)