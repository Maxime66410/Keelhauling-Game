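; BP_BasicCharacters is an AI character that takes on one of five pirate-themed skins and a starting side.
; ReceiveData swaps the skeletal mesh and anim class to match the skin and toggles the Hat's visibility.
; It then teleports the character to the BP_PointStart whose enum matches the IsOtherSide flag and stores that point.
; The AI move-to calls toward the stored point are disconnected and never run.
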(event Custom|ReceiveData
  (params (Skin :type SkinTypes%20Enum :default "NewEnumerator0") (IsOtherSide? :type Boolean))
  (bind _mesh (Variables|Character|GetMesh))
  (bind _mesh_2 (Variables|Character|GetMesh))
  (bind _mesh_3 (Variables|Character|GetMesh))
  (bind _mesh_4 (Variables|Character|GetMesh))
  (bind _mesh_5 (Variables|Character|GetMesh))
  (bind _hat (Variables|Default|GetHat))
  (bind _output_get (Variables|Default|SetSkinTypes Skin))
  (switch Utilities|FlowControl|Switch|SwitchonSkinTypes _output_get
    (:NewEnumerator0
      (Class|SkinnedMeshComponent|SetSkeletalMesh _mesh_2 "/Game/Assets/Model/Character/Deckhand/Deckhand_UE.Deckhand_UE" true)
      (Class|SkeletalMeshComponent|SetAnimClass _mesh_2 "/Game/Assets/Animation/Character/Deckhand/AB_Deckhand.AB_Deckhand_C")
      (Rendering|SetVisibility _hat true false))
    (:NewEnumerator1
      (Class|SkinnedMeshComponent|SetSkeletalMesh _mesh_3 "/Game/Assets/Model/Character/Wench/Wench_UE.Wench_UE" true)
      (Class|SkeletalMeshComponent|SetAnimClass _mesh_3 "/Game/Assets/Animation/Character/Wench/AB_Wench.AB_Wench_C")
      (Rendering|SetVisibility _hat true false))
    (:NewEnumerator2
      (Class|SkinnedMeshComponent|SetSkeletalMesh _mesh_4 "/Game/Content/ModularSkeletonArmy/CharacterParts_Skeleton/Meshes/Skeleton/SK_ma_skeleton_base.SK_ma_skeleton_base" true)
      (Class|SkeletalMeshComponent|SetAnimClass _mesh_4 "/Game/Content/ModularSkeletonArmy/Base/Animations/ABP_ma.ABP_ma_C")
      (Rendering|SetVisibility _hat false false))
    (:NewEnumerator3
      (Class|SkinnedMeshComponent|SetSkeletalMesh _mesh_5 "/Game/Assets/Model/Character/OldSeaDog/OldSeaDog_UE.OldSeaDog_UE" true)
      (Class|SkeletalMeshComponent|SetAnimClass _mesh_5 "/Game/Assets/Animation/Character/OldSeaDog/AB_OldSeaDog.AB_OldSeaDog_C")
      (Rendering|SetVisibility _hat false false))
    (:NewEnumerator4
      (Class|SkinnedMeshComponent|SetSkeletalMesh _mesh "/Game/Assets/Model/Character/Pirate/Pirate_UE.Pirate_UE" true)
      (Class|SkeletalMeshComponent|SetAnimClass _mesh "/Game/Assets/Animation/Character/Pirate/AB_Pirate.AB_Pirate_C")
      (Rendering|SetVisibility _hat true false)))
  (if IsOtherSide?
    (bind _outactors (Actor|GetAllActorsOfClass "/Game/Assets/Blueprint/AI/Spawn/BP_PointStart.BP_PointStart_C"))
    (bind _array_element (Utilities|Array|ForEachLoopwithBreak _outactors)
      (:LoopBody
        (if (Utilities|Enum|Equal(Enum) (Variables|/Game/Assets/Blueprint/AI/Spawn/BP_PointStart.BP_PointStart_C|GetEnum _array_element) "NewEnumerator1")
          (Transformation|Teleport (Transformation|GetWorldLocation (Variables|/Game/Assets/Blueprint/AI/Spawn/BP_PointStart.BP_PointStart_C|GetDefaultSceneRoot _array_element)) "0, 0, 0")
          (Variables|Default|SetArray%20Element _array_element)))
      (:Completed))
    (else
      (bind _outactors_2 (Actor|GetAllActorsOfClass "/Game/Assets/Blueprint/AI/Spawn/BP_PointStart.BP_PointStart_C"))
      (bind _array_element_2 (Utilities|Array|ForEachLoopwithBreak _outactors_2)
        (:LoopBody
          (if (Utilities|Enum|Equal(Enum) (Variables|/Game/Assets/Blueprint/AI/Spawn/BP_PointStart.BP_PointStart_C|GetEnum _array_element_2) "NewEnumerator0")
            (Transformation|Teleport (Transformation|GetWorldLocation (Variables|/Game/Assets/Blueprint/AI/Spawn/BP_PointStart.BP_PointStart_C|GetDefaultSceneRoot _array_element_2)) "0, 0, 0")
            (Variables|Default|SetArray%20Element _array_element_2)))
        (:Completed)))))

(event EventBeginPlay)

(fn ConstructionScript)